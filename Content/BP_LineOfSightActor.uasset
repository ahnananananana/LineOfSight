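; Line-of-sight actor that renders its visible view cone into a render target and publishes its position to a material parameter collection.
; A radius-synced sphere feeds overlapping actors' static meshes to AddAdjMesh/RemoveAdjMesh.
; Each tick, cone points come from GetDetectedPoints when optimized, otherwise from a fan of visibility traces, pushed outward by an offset.
; The points become an actor-centered triangle fan, drawn white on the cleared canvas at half world scale.
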(event `self.ReceiveBeginPlay`
  (bind _sphere (`self.Sphere`))
  (`SphereComponent.SetSphereRadius` _sphere (`self.m_dTraceLength`) true)
  (add `PrimitiveComponent.OnComponentBeginOverlap` _sphere (delegate `OnComponentBeginOverlap_Event_0`))
  (add `PrimitiveComponent.OnComponentEndOverlap` _sphere (delegate `OnComponentEndOverlap_Event_0`))
  (for _array_element (`PrimitiveComponent.GetOverlappingActors` _sphere null)
    (`self.AddAdjMesh` (`self.GetComponentByClass` _array_element "/Script/Engine.StaticMeshComponent"))))

(event `OnComponentEndOverlap_Event_0`
  (params (OverlappedComponent :type "PrimitiveComponent Object Reference") (OtherActor :type "Actor Object Reference") (OtherComp :type "PrimitiveComponent Object Reference") (OtherBodyIndex :type Integer))
  (`self.RemoveAdjMesh` (`self.GetComponentByClass` OtherActor "/Script/Engine.StaticMeshComponent")))

(event `OnComponentBeginOverlap_Event_0`
  (params (OverlappedComponent :type "PrimitiveComponent Object Reference") (OtherActor :type "Actor Object Reference") (OtherComp :type "PrimitiveComponent Object Reference") (OtherBodyIndex :type Integer) (bFromSweep :type Boolean) (SweepResult :type "HitResult Structure (by ref)"))
  (`self.AddAdjMesh` (`self.GetComponentByClass` OtherActor "/Script/Engine.StaticMeshComponent")))

(event `self.ReceiveTick`
  (params (DeltaSeconds :type "Float (single-precision)"))
  (bind _los_rendertarget (`self.LoS_RenderTarget`))
  (`SphereComponent.SetSphereRadius` (`self.Sphere`) (`self.m_dTraceLength`) false)
  (`|ExecutionSequence`
    (:`then_0`
      (`KismetMaterialLibrary.SetVectorParameterValue` "/Game/MPC_LineOfSight.MPC_LineOfSight" "ActorPosition" (`KismetMathLibrary.Conv_VectorToLinearColor` (`self.K2_GetActorLocation`))))
    (:`then_1`
      (`self.CreateCone`))
    (:`then_2`
      (`self.PrepareTrianglesForCanvas`))
    (:`then_3`
      (`KismetRenderingLibrary.ClearRenderTarget2D` _los_rendertarget (struct :`R` 0.25 :`G` 0.25 :`B` 0.25 :`A` 0.5))
      (bind (_canvas _size _context) (`KismetRenderingLibrary.BeginDrawCanvasToRenderTarget` _los_rendertarget))
      (`Canvas.K2_DrawTriangle` _canvas null (`self.CanvasTriangles`))
      (`KismetRenderingLibrary.EndDrawCanvasToRenderTarget` _context))))

(fn `CreateCone`
  (locals (`Angle Per Trace` :type "Float (double-precision)") (`Left Trace Vector` :type "Vector Structure" :default (0.0 0.0 0.0)))
  (bind _returnvalue (`self.K2_GetActorLocation`))
  (bind _m_itracecount (`self.m_iTraceCount`))
  (`KismetArrayLibrary.Array_Clear` (`self.TraceResults`))
  (if (`self.m_bIsOptimize`)
    (bind _returnvalue_2 (`self.GetDetectedPoints`))
    (for _array_element _returnvalue_2
      (bind _returnvalue_3 (* (`KismetMathLibrary.GreaterGreater_VectorRotator` (`local.Left Trace Vector`) (`KismetMathLibrary.MakeRotator` 0.0 0.0 (* (stale _index) (`local.Angle Per Trace`)))) (`self.m_dTraceLength`)))
      (bind _returnvalue_4 (+ (`self.K2_GetActorLocation`) _returnvalue_3))
      (`KismetArrayLibrary.Array_Add` (`self.TraceResults`) (select `bool` (`self.m_bIsOptimize`) :`false` (+ (select `bool` (stale _returnvalue_5) :`false` _returnvalue_4 :`true` (`.Location` (`GameplayStatics.BreakHitResult` (stale _outhit)))) (* (`KismetMathLibrary.Normal` _returnvalue_3) (`self.m_dTraceOffset`))) :`true` (+ (break `MeshPoint` _array_element) (* (`KismetMathLibrary.Normal` (- (break `MeshPoint` _array_element) _returnvalue)) (`self.m_dTraceOffset`)))) :!label _label))
    (else
      ;[1 1 1] Not Optimized
      (set `local.Left Trace Vector` (`KismetMathLibrary.GreaterGreater_VectorRotator` (`self.GetActorForwardVector`) (`KismetMathLibrary.MakeRotator` 0.0 0.0 (/ (`self.m_dViewAngle`) -2.0))))
      (set `local.Angle Per Trace` (/ (`self.m_dViewAngle`) _m_itracecount))
      (for _index (range (+ _m_itracecount 1))
        (bind (_outhit _returnvalue_5) (`KismetSystemLibrary.LineTraceSingle` :`Start` _returnvalue :`End` _returnvalue_4 :`TraceChannel` "TraceTypeQuery1" :`DrawDebugType` (select `bool` (`self.m_bIsShowTraceDebug`) :`true` "ForOneFrame" :!type "EDrawDebugTrace Enum")))
        (goto _label)))))

(fn `PrepareTrianglesForCanvas`
  (bind _returnvalue (`self.K2_GetActorLocation`))
  (bind _returnvalue_2 (`KismetMathLibrary.MakeVector` 1024.0 1024.0))
  (bind _traceresults (`self.TraceResults`))
  (bind _returnvalue_3 (`KismetMathLibrary.Conv_TransformToMatrix` (`KismetMathLibrary.MakeTransform` (0.0 0.0 0.0))))
  (`KismetArrayLibrary.Array_Clear` (`self.CanvasTriangles`))
  (for _index (range (+ (- (`KismetArrayLibrary.Array_Length` (`self.TraceResults`)) 2) 1))
    (`KismetArrayLibrary.Array_Add` (`self.CanvasTriangles`) (make `CanvasUVTri` (`KismetMathLibrary.Conv_VectorToVector2D` _returnvalue_2) (0.0 0.0) (struct :`R` 1.0 :`G` 1.0 :`B` 1.0 :`A` 1.0) (`KismetMathLibrary.Conv_VectorToVector2D` (+ (`KismetMathLibrary.Matrix_TransformVector` _returnvalue_3 (/ (- (`|GetArrayItem` _traceresults _index) _returnvalue) 2.0)) _returnvalue_2)) (0.0 0.0) (struct :`R` 1.0 :`G` 1.0 :`B` 1.0 :`A` 1.0) (`KismetMathLibrary.Conv_VectorToVector2D` (+ (`KismetMathLibrary.Matrix_TransformVector` _returnvalue_3 (/ (- (`|GetArrayItem` _traceresults (+ _index 1)) _returnvalue) 2.0)) _returnvalue_2)) (0.0 0.0) (struct :`R` 1.0 :`G` 1.0 :`B` 1.0 :`A` 1.0)))))

(fn `UserConstructionScript`)